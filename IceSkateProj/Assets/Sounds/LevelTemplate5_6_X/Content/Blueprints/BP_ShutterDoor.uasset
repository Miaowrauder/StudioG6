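; Shutter door Blueprint with red and green indicator lights, a timeline-driven door movement and a destruction event.
; LightSwitch turns the green light on and the red off, while Fall plays the DoorOpen timeline, whose Height track drives the door's Z scale with X and Y set to zero.
; Destroy plays a fracture sound at world origin and removes the Door, Light and Shutter components.
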(event Custom|Fall
  (bind _height (Timeline|DoorOpen Play)
    (:Update
      (Transformation|SetRelativeScale3D (Variables|Default|GetDoor) (Math|Vector|MakeVector 0.0 0.0 _height)))))

(event Custom|LightSwitch
  (Rendering|Components|Light|SetIntensity (Variables|Default|GetGreen) 1e+05)
  (Rendering|Components|Light|SetIntensity (Variables|Default|GetRed) 0.0))

(event Custom|Destroy
  (Audio|PlaySoundatLocation "/Game/SFX/Fracture2.Fracture2" "0, 0, 0" "0, 0, 0" 1.0 1.0 0.0 0 0 0 0)
  (Components|DestroyComponent (Variables|Default|GetDoor)))

(fn ConstructionScript)