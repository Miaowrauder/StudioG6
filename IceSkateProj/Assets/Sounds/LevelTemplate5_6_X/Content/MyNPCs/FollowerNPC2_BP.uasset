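; A follower NPC that chases the first-person player until served, then waits to deliver story dialogue.
; Before being served, Tick turns it toward the player and re-issues AI MoveTo; afterwards, while waiting, a timer replays pleading text and ghost audio.
; The End event walks it to a fixed spot, where player overlap stops the pleas, shows lore about oracular paintings and activates CrossMesh_BP.
; Kill swaps it for a breakable body.
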(event OnComponentBeginOverlap(Sphere)
  (params (OverlappedComponent :type Primitive%20Component%20Object%20Reference) (OtherActor :type Actor%20Object%20Reference) (OtherComp :type Primitive%20Component%20Object%20Reference) (OtherBodyIndex :type Integer) (bFromSweep :type Boolean) (SweepResult :type Hit%20Result%20Structure%20%28by%20ref%29))
  (if (and (Utilities|String|Contains (Utilities|GetDisplayName OtherActor) "FirstPerson") (Variables|Default|Getserved?))
    (Utilities|FlowControl|DoOnce false
      (:Completed
        (Variables|Default|Setwaiting false)
        (Audio|PlaySoundatLocation "/Game/VoiceLines/HorseofWisdomWhimsy/ghost4.ghost4" (Math|Vector|MakeVector -4522.0 7374.0 6e+01) "0, 0, 0" 1.0 1.0 0.0 0 0 0 0)
        (Rendering|Components|TextRender|SetText (Variables|Default|GetTextRender) (Utilities|Text|ToText(String) "The oracular paintings from long ago..."))
        (Utilities|FlowControl|Delay 2.0)
        (Rendering|Components|TextRender|SetText (Variables|Default|GetTextRender) (Utilities|Text|ToText(String) "They hold the secrets to loam restoration..."))
        (bind _returnvalue (Actor|GetActorOfClass "/Game/CrossMesh_BP.CrossMesh_BP_C"))
        (Default|Activate _returnvalue)))))

(event Custom|End
  (AI|AIMoveTo (AI|GetAIController (Pawn|GetController)) (Math|Vector|MakeVector -4522.0 7374.0 6e+01) 0 -1.0 "Default" "Default" true true
    (:OnMoveFinished
      (Transformation|SetActorRotation "0.000000,5.000000,0.000000")
      (Audio|PlaySoundatLocation "/Game/VoiceLines/HorseofWisdomWhimsy/ghost5.ghost5" "0, 0, 0" "0, 0, 0" 1.0 1.0 0.0 0 0 0 0))))

(event Custom|PlayRepeat
  (Rendering|Components|TextRender|SetText (Variables|Default|GetTextRender) (Utilities|Text|ToText(String) "please..."))
  (Audio|PlaySoundatLocation "/Game/VoiceLines/HorseofWisdomWhimsy/ghost6.ghost6" "0, 0, 0" "0, 0, 0" 1.0 1.0 0.0 0 0 0 0)
  (Utilities|FlowControl|Delay 0.4)
  (Rendering|Components|TextRender|SetText (Variables|Default|GetTextRender) (Utilities|Text|ToText(String) "come..."))
  (Utilities|FlowControl|Delay 0.4)
  (Rendering|Components|TextRender|SetText (Variables|Default|GetTextRender) (Utilities|Text|ToText(String) "we don't have long..."))
  (Variables|Default|SetwaitTimer 1e+01)
  (Utilities|FlowControl|DoOnce false) ; enters at Reset
)

(event EventTick
  (params (DeltaSeconds :type Float%20%28single-precision%29))
  (if (!= (Variables|Default|Getserved?) true)
    (bind _returnvalue (Actor|GetActorOfClass "/Game/FirstPersonBP1/Blueprints/BP_FirstPersonCharacter.BP_FirstPersonCharacter_C"))
    (bind _output_get (Variables|Default|SetplayerBP _returnvalue))
    (Transformation|SetActorRotation (Math|Conversions|RotationFromXVector (- (Transformation|GetActorLocation _output_get) (Transformation|GetActorLocation))))
    (Utilities|FlowControl|DoOnce false :!label _label
      (:Completed
        (AI|AIMoveTo (AI|GetAIController (Pawn|GetController)) "0, 0, 0" _output_get 2.5e+02 "Default" "Default" true true
          (:OnMoveFinished
            (goto _label Reset)))))
    (elif (Variables|Default|Getwaiting)
      (if (> (Variables|Default|GetwaitTimer) 0.0)
        (Variables|Default|SetwaitTimer (- (Variables|Default|GetwaitTimer) DeltaSeconds))
        (else
          (Utilities|FlowControl|DoOnce false
            (:Completed
              (CallFunction|PlayRepeat))))))))

(fn ConstructionScript)

(fn Kill
  (Utilities|String|LogString "KILLL!")
  (bind _returnvalue (Game|SpawnActorfromClass "/Game/Meshes/BreakableManInnit.BreakableManInnit_C" (Transformation|GetActorTransform) "AlwaysSpawn" "MultiplyWithRoot" 0 0))
  (Default|Death _returnvalue)
  (Actor|DestroyActor))