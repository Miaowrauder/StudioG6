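; BP_LazerPuzzle is a six-button sequence puzzle that opens the way through BP_LazerDoor.
; Component hits append to TempButtons, which is checked against the order of the Cube's child components.
; Correct presses shift buttons along world X, apply glow materials and play sounds; a wrong one resets everything.
; Completion deactivates the buttons and, inside that same loop, calls the door's Fall and LightSwitch and plays a jingle.
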(event OnComponentHit(5)
  (params (HitComponent :type Primitive%20Component%20Object%20Reference) (OtherActor :type Actor%20Object%20Reference) (OtherComp :type Primitive%20Component%20Object%20Reference) (NormalImpulse :type Vector :default "0, 0, 0") (Hit :type Hit%20Result%20Structure%20%28by%20ref%29))
  (CallFunction|AddButton HitComponent))

(event OnComponentHit(2)
  (params (HitComponent :type Primitive%20Component%20Object%20Reference) (OtherActor :type Actor%20Object%20Reference) (OtherComp :type Primitive%20Component%20Object%20Reference) (NormalImpulse :type Vector :default "0, 0, 0") (Hit :type Hit%20Result%20Structure%20%28by%20ref%29))
  (CallFunction|AddButton HitComponent))

(event OnComponentHit(4)
  (params (HitComponent :type Primitive%20Component%20Object%20Reference) (OtherActor :type Actor%20Object%20Reference) (OtherComp :type Primitive%20Component%20Object%20Reference) (NormalImpulse :type Vector :default "0, 0, 0") (Hit :type Hit%20Result%20Structure%20%28by%20ref%29))
  (CallFunction|AddButton HitComponent))

(event OnComponentHit(1)
  (params (HitComponent :type Primitive%20Component%20Object%20Reference) (OtherActor :type Actor%20Object%20Reference) (OtherComp :type Primitive%20Component%20Object%20Reference) (NormalImpulse :type Vector :default "0, 0, 0") (Hit :type Hit%20Result%20Structure%20%28by%20ref%29))
  (CallFunction|AddButton HitComponent))

(event OnComponentHit(3)
  (params (HitComponent :type Primitive%20Component%20Object%20Reference) (OtherActor :type Actor%20Object%20Reference) (OtherComp :type Primitive%20Component%20Object%20Reference) (NormalImpulse :type Vector :default "0, 0, 0") (Hit :type Hit%20Result%20Structure%20%28by%20ref%29))
  (CallFunction|AddButton HitComponent))

(event OnComponentHit(6)
  (params (HitComponent :type Primitive%20Component%20Object%20Reference) (OtherActor :type Actor%20Object%20Reference) (OtherComp :type Primitive%20Component%20Object%20Reference) (NormalImpulse :type Vector :default "0, 0, 0") (Hit :type Hit%20Result%20Structure%20%28by%20ref%29))
  (CallFunction|AddButton HitComponent))

(event Custom|AddButton
  (params (Button :type Primitive%20Component%20Object%20Reference))
  (Utilities|Array|Add (Variables|Default|GettempButtons) Button)
  (CallFunction|CheckButtons))

(event Custom|CheckButtons
  (if true
    (bind (_array_element _array_index) (Utilities|Array|ForEachLoopwithBreak (Variables|Default|GettempButtons) :!label _label)
      (:LoopBody
        (if (== _array_element (Utilities|Array|Get(acopy) (Variables|Default|GetButtons) _array_index))
          (if (== (+ _array_index 1) (Utilities|Array|Length (Variables|Default|GettempButtons)))
            (Audio|PlaySoundatLocation (Utilities|Array|Get(acopy) (Variables|Default|GetButtonSFX) _array_index) "0, 0, 0" "0, 0, 0" 1.0 1.0 0.0 0 0 0 0))
          (Transformation|SetWorldLocation (Utilities|Array|Get(acopy) (Variables|Default|GetButtons) _array_index) (Math|Vector|MakeVector 3917.0 (.y (Transformation|GetWorldLocation (Utilities|Array|Get(acopy) (Variables|Default|GetButtons) _array_index))) (.z (Transformation|GetWorldLocation (Utilities|Array|Get(acopy) (Variables|Default|GetButtons) _array_index)))) false false)
          (Rendering|Material|SetMaterial (Utilities|Array|Get(acopy) (Variables|Default|GetButtonMeshes) _array_index) 0 (Utilities|Array|Get(acopy) (Variables|Default|GetGlowMats) _array_index))
          (if (== _array_index 5)
            (CallFunction|Complete))
          (else
            (CallFunction|ResetButton)
            (goto _label Break)))))))

(event Custom|ResetButton
  (for (_array_element _array_index) (Variables|Default|GetButtons)
    (Transformation|SetWorldLocation _array_element (Math|Vector|MakeVector 3897.0 (.y (Transformation|GetWorldLocation _array_element)) (.z (Transformation|GetWorldLocation _array_element))) false false)
    (Rendering|Material|SetMaterial (Utilities|Array|Get(acopy) (Variables|Default|GetButtonMeshes) _array_index) 0 (Utilities|Array|Get(acopy) (Variables|Default|GetFlatMats) _array_index)))
  (Utilities|Array|Clear (Variables|Default|GettempButtons))
  (Audio|PlaySoundatLocation "/Game/SFX/WrongButton.WrongButton" "0, 0, 0" "0, 0, 0" 9.0 1.0 0.0 0 0 0 0))

(event Custom|Complete
  (Development|PrintString "Done")
  (for _array_element (Variables|Default|GetButtons)
    (Components|Activation|SetActive _array_element false false)
    (bind _returnvalue (Actor|GetActorOfClass "/Game/Blueprints/BP_LazerDoor.BP_LazerDoor_C"))
    (Default|Fall _returnvalue)
    (Default|LightSwitch _returnvalue)
    (Audio|PlaySoundatLocation "/Game/Music/The_Price_is_Right.The_Price_is_Right" "0, 0, 0" "0, 0, 0" 0.5 1.0 0.0 0 0 0 0)))

(event Collision|EventActorBeginOverlap
  (params (OtherActor :type Actor%20Object%20Reference)))

(event EventTick
  (params (DeltaSeconds :type Float%20%28single-precision%29)))

(event EventBeginPlay
  (Variables|Default|SetGlowMats (Utilities|Array|MakeArray "/Game/Materials/M_DarkRedGlow.M_DarkRedGlow" "/Game/Materials/M_GlowOrange1.M_GlowOrange1" "/Game/Materials/M_GlowDarkGreyNavy.M_GlowDarkGreyNavy" "/Game/Materials/M_Glow_Yellow.M_Glow_Yellow" "/Game/Materials/M_BlueGlow.M_BlueGlow" "/Game/Materials/M_GlowPurple1.M_GlowPurple1"))
  (Variables|Default|SetFlatMats (Utilities|Array|MakeArray "/Game/Materials/M_Flat_Red.M_Flat_Red" "/Game/Materials/M_FlatOrange.M_FlatOrange" "/Game/Materials/M_FlatGreen.M_FlatGreen" "/Game/Materials/M_Flat_Yellow.M_Flat_Yellow" "/Game/Materials/M_FlatBlue.M_FlatBlue" "/Game/Materials/M_FlatPurple.M_FlatPurple"))
  (Variables|Default|SetButtonMeshes (Utilities|Array|MakeArray (Variables|Default|Get1) (Variables|Default|Get2) (Variables|Default|Get3) (Variables|Default|Get4) (Variables|Default|Get5) (Variables|Default|Get6)))
  (Variables|Default|SetButtonSFX (Utilities|Array|MakeArray "/Game/SFX/Button1.Button1" "/Game/SFX/Button2.Button2" "/Game/SFX/Button3.Button3" "/Game/SFX/Button4.Button4" "/Game/SFX/Button5.Button5"))
  (Variables|Default|SetButtons (Components|GetChildrenComponents (Variables|Default|GetCube) false)))

(fn ConstructionScript)