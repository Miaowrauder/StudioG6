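; BP_Basket is a weighing basket that tracks the total mass of fruit placed inside its box.
; Box overlaps add or subtract each fruit's mass, using the Tube_Blueprint's Inside Z scale as both stored total and fill level, capped on entry, and update its kg text.
; Fruit is identified by display name, the crane only prints a debug message, and CallED1 fires when the weight nearly equals 2 kg.
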(event OnComponentBeginOverlap(Box)
  (params (OverlappedComponent :type Primitive%20Component%20Object%20Reference) (OtherActor :type Actor%20Object%20Reference) (OtherComp :type Primitive%20Component%20Object%20Reference) (OtherBodyIndex :type Integer) (bFromSweep :type Boolean) (SweepResult :type Hit%20Result%20Structure%20%28by%20ref%29))
  (if (Utilities|Enum|Equal(Enum) (Utilities|GetDisplayName OtherActor) "CraneBP")
    (Development|PrintString "CRANE!")
    (else
      (bind _asprimitive_component (Utilities|Casting|CastToPrimitiveComponent (Variables|/Script/Engine.Actor|GetRootComponent OtherActor)))
      (if (Utilities|String|Contains (Utilities|GetDisplayName OtherActor) "Fruit") ; other object a fruit?
        (bind _returnvalue (Actor|GetActorOfClass "/Game/Blueprints/Tube_Blueprint.Tube_Blueprint_C"))
        (bind _output_get (Variables|Default|SetMass (Physics|GetMass _asprimitive_component)))
        (bind _output_get_2 (Variables|Default|SetWeight (.z (Transformation|GetWorldScale (Variables|/Game/Blueprints/Tube_Blueprint.Tube_Blueprint_C|GetInside _returnvalue)))))
        (Variables|Default|SetScale (Variables|/Game/Blueprints/Tube_Blueprint.Tube_Blueprint_C|GetInside _returnvalue))
        (Variables|Default|SetMassText (Variables|/Game/Blueprints/Tube_Blueprint.Tube_Blueprint_C|GetMass _returnvalue))
        (if (>= (+ _output_get _output_get_2) 2.75) ; is new weight the max?
          (Variables|Default|SetWeight (+ _output_get _output_get_2)) ; cap it at max
          (Transformation|SetWorldScale3D (Variables|Default|GetScale) (Math|Vector|MakeVector (.x (Transformation|GetWorldScale (Variables|Default|GetScale))) (.y (Transformation|GetWorldScale (Variables|Default|GetScale))) 2.75))
          (else
            (bind _output_get_3 (Variables|Default|SetWeight (+ _output_get _output_get_2))) ; add new weight
            (Transformation|SetWorldScale3D (Variables|Default|GetScale) (Math|Vector|MakeVector (.x (Transformation|GetWorldScale (Variables|Default|GetScale))) (.y (Transformation|GetWorldScale (Variables|Default|GetScale))) _output_get_3))))
        (Rendering|Components|TextRender|SetText (Variables|Default|GetMassText) (Utilities|Text|ToText(String) (Class|KismetStringLibrary|BuildStringDouble "" "" (Variables|Default|GetWeight) " kg")))
        (if (Math|Float|NearlyEqual(Float) (Variables|Default|GetWeight) 2.0 1e-06)
          (Default|CallED1))))))

(event OnComponentEndOverlap(Box)
  (params (OverlappedComponent :type Primitive%20Component%20Object%20Reference) (OtherActor :type Actor%20Object%20Reference) (OtherComp :type Primitive%20Component%20Object%20Reference) (OtherBodyIndex :type Integer))
  (bind _asprimitive_component (Utilities|Casting|CastToPrimitiveComponent (Variables|/Script/Engine.Actor|GetRootComponent OtherActor)))
  (if (Utilities|String|Contains (Utilities|GetDisplayName OtherActor) "Fruit") ; is fruit?
    (bind _returnvalue (Actor|GetActorOfClass "/Game/Blueprints/Tube_Blueprint.Tube_Blueprint_C"))
    (bind _output_get (Variables|Default|SetMass (Physics|GetMass _asprimitive_component)))
    (bind _output_get_2 (Variables|Default|SetWeight (.z (Transformation|GetWorldScale (Variables|/Game/Blueprints/Tube_Blueprint.Tube_Blueprint_C|GetInside _returnvalue)))))
    (Variables|Default|SetScale (Variables|/Game/Blueprints/Tube_Blueprint.Tube_Blueprint_C|GetInside _returnvalue))
    (Variables|Default|SetMassText (Variables|/Game/Blueprints/Tube_Blueprint.Tube_Blueprint_C|GetMass _returnvalue))
    (bind _output_get_3 (Variables|Default|SetWeight (- _output_get_2 _output_get))) ; minus mass from weight
    (Transformation|SetWorldScale3D (Variables|Default|GetScale) (Math|Vector|MakeVector (.x (Transformation|GetWorldScale (Variables|Default|GetScale))) (.y (Transformation|GetWorldScale (Variables|Default|GetScale))) _output_get_3))
    (Rendering|Components|TextRender|SetText (Variables|Default|GetMassText) (Utilities|Text|ToText(String) (Class|KismetStringLibrary|BuildStringDouble "" "" (Variables|Default|GetWeight) " kg")))
    (if (Math|Float|NearlyEqual(Float) (Variables|Default|GetWeight) 2.0 1e-06)
      (Default|CallED1))))

(fn ConstructionScript)