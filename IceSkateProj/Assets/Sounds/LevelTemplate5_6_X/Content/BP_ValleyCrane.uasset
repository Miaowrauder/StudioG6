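; Valley crane that carries a fruit basket along a spline and drops it as a pickup.
; It finds the Path1 actor named CranePath, then ToLeft and ToRight check IsRight and use timelines to slide Cube1 along its spline.
; Finishing the ToLeft move calls CallEDCrane.
; Grab reveals the hidden basket and hook meshes, while Release hides them and spawns BP_BasketPickup at the basket's location.
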(event Custom|To%20Right
  (bind _array_element_0 (Variables|Default|GetArray%20Element_0))
  (bind _spline (Variables|/Game/MyNPCs/HorseofWisdomandWhimsy/Path1.Path1_C|GetSpline _array_element_0))
  (if (not (Variables|Default|GetisRight))
    (bind _move (Timeline|Timeline_0 ReverseFromEnd)
      (:Update
        (Transformation|SetWorldLocation (Variables|Default|GetCube1) (.location (Spline|GetTransformatDistanceAlongSpline _spline (Math|Float|Lerp 0.0 (Spline|GetSplineLength _spline) _move) "World" false)) false false)))))

(event Custom|To%20Left
  (bind _array_element_0 (Variables|Default|GetArray%20Element_0))
  (bind _spline (Variables|/Game/MyNPCs/HorseofWisdomandWhimsy/Path1.Path1_C|GetSpline _array_element_0))
  (if (Variables|Default|GetisRight)
    (bind _move (Timeline|Timeline Play)
      (:Update
        (Transformation|SetWorldLocation (Variables|Default|GetCube1) (.location (Spline|GetTransformatDistanceAlongSpline _spline (Math|Float|Lerp 0.0 (Spline|GetSplineLength _spline) _move) "World" false)) false false))
      (:Finished
        (Default|CallEDCrane)))))

(event Custom|Grab
  (params (NewParam :type Scene%20Component%20Object%20Reference))
  (Rendering|SetVisibility (Variables|Default|GetSphere) true false))

(event Custom|Release
  (Rendering|SetVisibility (Variables|Default|GetBox) false false)
  (Game|SpawnActorfromClass "/Game/Blueprints/BP_BasketPickup.BP_BasketPickup_C" (Math|Transform|MakeTransform (Transformation|GetWorldLocation (Variables|Default|GetBasket)) "0, 0, 0" "1.000000,1.000000,1.000000") "Undefined" "MultiplyWithRoot" 0 0))

(event Custom|CustomEvent_1
  (bind _returnvalue (Actor|GetActorOfClass "/Game/BP_CLAW.BP_CLAW_C"))
  (Variables|Default|SetNewVar _returnvalue)
  (bind _outactors (Actor|GetAllActorsOfClass "/Game/MyNPCs/HorseofWisdomandWhimsy/Path1.Path1_C"))
  (for _array_element _outactors
    (if (Utilities|Enum|Equal(Enum) (Utilities|GetDisplayName _array_element) "CranePath")
      (Variables|Default|SetArray%20Element_0 _array_element))))

(event EventBeginPlay
  (Rendering|SetVisibility (Variables|Default|GetSphere) false false)
  (bind _outactors (Actor|GetAllActorsOfClass "/Game/MyNPCs/HorseofWisdomandWhimsy/Path1.Path1_C"))
  (for _array_element _outactors
    (if (Utilities|Enum|Equal(Enum) (Utilities|GetDisplayName _array_element) "CranePath")
      (Variables|Default|SetArray%20Element_0 _array_element))))

(fn ConstructionScript)