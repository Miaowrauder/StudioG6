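; Cutscene ghost that descends to deliver a crane instruction to the player, then replaces itself with a follower NPC.
; Descend plays a sound and moves it along the Path spline by timeline, then shows the text, calls the player's CanMove and swaps in FollowerNPC_BP.
; Tick keeps it facing the player and would chase them from Stage 2, never set here.
; Kill swaps it for a BreakableManInnit and triggers its Death.
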(event Custom|Descend
  (bind _path (Variables|Default|GetPath))
  (bind _spline (Variables|/Game/MyNPCs/HorseofWisdomandWhimsy/Path1.Path1_C|GetSpline _path))
  (Audio|PlaySoundatLocation "/Game/VoiceLines/HorseofWisdomWhimsy/ghost1.ghost1" (Transformation|GetActorLocation) "0, 0, 0" 1.0 1.0 0.0 0 0 0 0)
  (bind _horse (Timeline|Timeline Play)
    (:Update
      (Transformation|SetActorLocation (.location (Spline|GetTransformatDistanceAlongSpline _spline (Math|Float|Lerp 0.0 (Spline|GetSplineLength _spline) _horse) "World" false)) false false))
    (:Finished
      (Utilities|FlowControl|Delay 2.0)
      (Variables|Default|SetStage 1)
      (CallFunction|PlayDialogue))))

(event Custom|PlayDialogue
  (if (== (Variables|Default|GetStage) 1)
    (Rendering|Components|TextRender|SetText (Variables|Default|GetTextRender) (Utilities|Text|ToText(String) "you need to use the crane to blend the holy produce..."))
    (Audio|PlaySoundatLocation "/Game/VoiceLines/HorseofWisdomWhimsy/ghost2.ghost2" (Transformation|GetActorLocation) "0, 0, 0" 1.0 1.0 0.0 0 0 0 0)
    (Utilities|FlowControl|Delay 2.0)
    (Default|CanMove (Variables|Default|GetPlayer))
    (Game|SpawnActorfromClass "/Game/MyNPCs/FollowerNPC_BP.FollowerNPC_BP_C" (Math|Transform|MakeTransform (.location (Transformation|GetActorTransform)) "0, 0, 0" "1.000000,1.000000,1.000000") "AdjustIfPossibleButAlwaysSpawn" "MultiplyWithRoot" 0 0)
    (Actor|DestroyActor)))

(event EventTick
  (params (DeltaSeconds :type Float%20%28single-precision%29))
  (bind _returnvalue (Actor|GetActorOfClass "/Game/FirstPersonBP1/Blueprints/BP_FirstPersonCharacter.BP_FirstPersonCharacter_C"))
  (bind _output_get (Variables|Default|SetPlayer _returnvalue))
  (if (>= (Variables|Default|GetStage) 2)
    (AI|Navigation|SimpleMovetoActor (Pawn|GetController) _output_get))
  (Transformation|SetActorRotation (Math|Conversions|RotationFromXVector (- (Transformation|GetActorLocation _output_get) (Transformation|GetActorLocation)))))

(fn ConstructionScript)

(fn Kill
  (Utilities|String|LogString "KILLL!")
  (bind _returnvalue (Game|SpawnActorfromClass "/Game/Meshes/BreakableManInnit.BreakableManInnit_C" (Transformation|GetActorTransform) "AlwaysSpawn" "MultiplyWithRoot" 0 0))
  (Default|Death _returnvalue)
  (Actor|DestroyActor))