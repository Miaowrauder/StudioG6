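; One-shot trigger box that starts a scripted HoWW encounter when the first-person player walks into it.
; On overlap it calls CantMove on the character, then finds the Path1 actor with display name "Horse2".
; It spawns a HoWW at that location, hands it the path and a line of harvest-themed text, calls Descend, then destroys itself.
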(event OnComponentBeginOverlap(CollisionComponent)
  (params (OverlappedComponent :type Primitive%20Component%20Object%20Reference) (OtherActor :type Actor%20Object%20Reference) (OtherComp :type Primitive%20Component%20Object%20Reference) (OtherBodyIndex :type Integer) (bFromSweep :type Boolean) (SweepResult :type Hit%20Result%20Structure%20%28by%20ref%29))
  (if (Utilities|String|Contains (Utilities|GetDisplayName OtherActor) "FirstPerson")
    (bind _asbp_first_person_character (Utilities|Casting|CastToBP_FirstPersonCharacter OtherActor))
    (Default|Can'tMove _asbp_first_person_character)
    (bind _outactors (Actor|GetAllActorsOfClass "/Game/MyNPCs/HorseofWisdomandWhimsy/Path1.Path1_C"))
    (for _array_element _outactors
      (if (Utilities|Enum|Equal(Enum) (Utilities|GetDisplayName _array_element) "Horse2")
        (bind _returnvalue (Game|SpawnActorfromClass "/Game/MyNPCs/HorseofWisdomandWhimsy/HoWW.HoWW_C" (Math|Transform|MakeTransform (Transformation|GetActorLocation _array_element) "0, 0, 0" "1.000000,1.000000,1.000000") "Undefined" "MultiplyWithRoot" 0 0))
        (Variables|/Game/MyNPCs/HorseofWisdomandWhimsy/HoWW.HoWW_C|SetPath _returnvalue _array_element)
        (Variables|/Game/MyNPCs/HorseofWisdomandWhimsy/HoWW.HoWW_C|Set1 _returnvalue "the harvest was indeed bountiful this year.... 
 
do not disappoint the loam...")
        (Default|Descend _returnvalue)
        (Actor|DestroyActor)))))

(fn ConstructionScript)