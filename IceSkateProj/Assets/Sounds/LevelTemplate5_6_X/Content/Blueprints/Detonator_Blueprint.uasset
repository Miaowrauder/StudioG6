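; Plunger detonator that inflates BP_Bomb until it explodes and breaks the Z3 walls.
; LightSwitch arms it, turning the light green.
; While armed, Tick limits handle height and converts vertical velocity into bomb scale: downward motion grows it, upward shrinks it to a floor.
; At the size threshold, it detaches the handle, plays Niagara and sound effects, destroys the bomb and spawns FS_MasterField at the geometry-collection walls to fracture them.
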(event Custom|LightSwitch
  (Rendering|Material|SetMaterial (Variables|Default|GetLight) 1 "/Game/Materials/M_GlowDarkGreyNavy.M_GlowDarkGreyNavy")
  (Rendering|Components|Light|SetIntensity (Variables|Default|GetGreenLight) 5e+04)
  (Rendering|Components|Light|SetIntensity (Variables|Default|GetRedLight) 0.0)
  (Variables|Default|Setmulched true))

(event Custom|Explode!
  (Audio|PlaySoundatLocation "/Game/SFX/Explosion.Explosion" "0, 0, 0" "0, 0, 0" 1.0 1.0 0.0 0 0 0 0)
  (Niagara|SpawnSystematLocation (Variables|Default|GetEXPLOSION) "-1996.467248,7639.702709,469.323791" "0, 0, 0" "30.000000,30.000000,30.000000")
  (Actor|DestroyActor (stale EventTick _returnvalue_4))
  (bind _returnvalue (Actor|GetActorOfClass "/Game/GC_Z3Walls_Blueprint.GC_Z3Walls_Blueprint_C"))
  (Game|SpawnActorfromClass "/Engine/EditorResources/FieldNodes/FS_MasterField.FS_MasterField_C" (Math|Transform|MakeTransform (Transformation|GetActorLocation _returnvalue) "0, 0, 0" "1.000000,1.000000,1.000000") "Undefined" "MultiplyWithRoot" 0 0)
  (Utilities|FlowControl|Delay 0.75)
  (Audio|PlaySoundatLocation "/Game/SFX/Fracture1.Fracture1" "0, 0, 0" "0, 0, 0" 1.0 1.0 0.0 0 0 0 0))

(event EventTick
  (params (DeltaSeconds :type Float%20%28single-precision%29))
  (bind _handle (Variables|Default|GetHandle))
  (bind _base (Variables|Default|GetBase))
  (bind _minhandleheight (Variables|Default|GetminHandleHeight))
  (bind _maxhandleheight (Variables|Default|GetmaxHandleHeight))
  (bind _returnvalue (Transformation|GetWorldLocation _handle))
  (bind _returnvalue_2 (Transformation|GetWorldLocation _base))
  (bind _returnvalue_3 (- (Math|Vector|MakeVector (.x _returnvalue) (.y _returnvalue) (.z _returnvalue)) _returnvalue_2))
  (if (Variables|Default|Getmulched)
    (if (not (Variables|Default|GetExploded))
      (if (<= (.z _returnvalue_3) _minhandleheight)
        (Transformation|SetWorldLocation _handle (Math|Vector|MakeVector (.x _returnvalue) (.y _returnvalue) _minhandleheight) false false)
        (elif (>= (.z _returnvalue_3) _maxhandleheight)
          (Transformation|SetWorldLocation _handle (Math|Vector|MakeVector (.x _returnvalue) (.y _returnvalue) _maxhandleheight) false false)))
      (if (> (+ (Variables|Default|GetbombSize) (/ (.z (Transformation|GetComponentVelocity _handle)) -1e+04)) 0.15)
        (bind _output_get (Variables|Default|SetbombSize (+ (Variables|Default|GetbombSize) (/ (.z (Transformation|GetComponentVelocity _handle)) -1e+04))))
        (else
          (Variables|Default|SetbombSize 0.15)))
      (bind _returnvalue_4 (Actor|GetActorOfClass "/Game/Blueprints/BP_Bomb.BP_Bomb_C"))
      (if (< (.z (.scale (Transformation|GetActorTransform _returnvalue_4))) 1.35)
        (Transformation|SetWorldTransform (Variables|/Script/Engine.Actor|GetRootComponent _returnvalue_4) (Math|Transform|MakeTransform (.location (Transformation|GetActorTransform _returnvalue_4)) (.rotation (Transformation|GetActorTransform _returnvalue_4)) (Math|Vector|MakeVector _output_get _output_get _output_get)) false false)
        (else
          (Variables|Default|SetExploded true)
          (Utilities|FlowControl|Delay 1.0)
          (Transformation|DetachFromComponent (Variables|Default|GetHandle) "KeepRelative" "KeepRelative" "KeepRelative" true)
          (CallFunction|Explode!))))))

(fn ConstructionScript)