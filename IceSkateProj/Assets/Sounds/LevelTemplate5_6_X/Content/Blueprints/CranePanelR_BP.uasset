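; Interactive crane control panel with Release, Grab and Move buttons that operates BP_ValleyCrane once activated.
; Highlight and Off swap button materials and text colors by ButtonIndex, using parallel mesh and text arrays.
; Interact calls the crane's action for that index, with grabbing gated by CanGrab and the crane being on the right.
; Move picks right or left by checking whether the panel's display name contains "RPanel".
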(event Custom|Highlight
  (if (Variables|Default|GetActive)
    (for (_array_element _array_index) (Variables|Default|GetButtonArr)
      (Utilities|IsValid _array_element
        (:Is%20Valid
          (if (== _array_index (Variables|Default|GetButtonIndex))
            (bind _output_get (Variables|Default|SetCurrentButton _array_element))
            (Rendering|Material|SetMaterial _output_get 0 "/Game/Materials/M_Glow_Yellow.M_Glow_Yellow")
            (Rendering|Components|TextRender|SetTextRenderColor (Utilities|Array|Get(acopy) (Variables|Default|GetTextArr) _array_index) (Variables|Default|GetSelected))
            (else
              (Rendering|Material|SetMaterial _array_element 0 "/Game/Materials/M_FlatBlackGloss.M_FlatBlackGloss")
              (Rendering|Components|TextRender|SetTextRenderColor (Utilities|Array|Get(acopy) (Variables|Default|GetTextArr) _array_index) (Variables|Default|GetUnselected)))))))))

(event Custom|Activate
  (bind _grab (Variables|Default|GetGrab))
  (Variables|Default|SetActive true)
  (Rendering|SetVisibility (Variables|Default|GetMoveCube) true false)
  (Rendering|Components|TextRender|SetText (Variables|Default|GetMove) (Utilities|Text|ToText(String) "Move"))
  (Rendering|Components|TextRender|SetText (Variables|Default|GetRelease) (Utilities|Text|ToText(String) "Release"))
  (Rendering|Components|TextRender|SetText _grab (Utilities|Text|ToText(String) "Grab"))
  (Rendering|Components|TextRender|SetTextRenderColor _grab (Variables|Default|GetUnselected)))

(event Custom|Off
  (if (Variables|Default|GetActive)
    (for (_array_element _array_index) (Variables|Default|GetButtonArr)
      (if (== _array_index (Variables|Default|GetButtonIndex))
        (Rendering|Material|SetMaterial _array_element 0 "/Game/Materials/M_FlatBlackGloss.M_FlatBlackGloss")
        (Rendering|Components|TextRender|SetTextRenderColor (Utilities|Array|Get(acopy) (Variables|Default|GetTextArr) _array_index) (Variables|Default|GetUnselected))))))

(event EventInteract
  (params (ActorObjectReference :type Actor%20Object%20Reference))
  (if (Variables|Default|GetActive)
    (bind _returnvalue (Actor|GetActorOfClass "/Game/BP_ValleyCrane.BP_ValleyCrane_C"))
    (Variables|Default|SetCrane _returnvalue)
    (if (== 0 (Variables|Default|GetButtonIndex))
      ;[0.15 0.15 0.15 0.5] Release!
      (Rendering|Material|SetMaterial (Variables|Default|GetReleaseCube) 0 "/Game/Materials/M_DarkRedGlow.M_DarkRedGlow")
      (Rendering|Components|TextRender|SetTextRenderColor (Variables|Default|GetRelease) (Variables|Default|GetSelected))
      (Default|Release (Variables|Default|GetCrane))
      (elif (== 1 (Variables|Default|GetButtonIndex))
        (if (Variables|Default|GetCanGrab)
          ;[0.15 0.15 0.15 0.5] Grab!
          (Rendering|Material|SetMaterial (Variables|Default|GetGrabCube) 0 "/Game/Materials/M_DarkRedGlow.M_DarkRedGlow")
          (Rendering|Components|TextRender|SetTextRenderColor (Variables|Default|GetGrab) (Variables|Default|GetSelected))
          (if (Variables|/Game/BP_ValleyCrane.BP_ValleyCrane_C|GetisRight (Variables|Default|GetCrane))
            (Default|Grab (Variables|Default|GetCrane))
            (Variables|Default|SethasObject? true)))
        (elif (== 2 (Variables|Default|GetButtonIndex))
          ;[0.15 0.15 0.15 0.5] Move!
          (Rendering|Material|SetMaterial (Variables|Default|GetMoveCube) 0 "/Game/Materials/M_DarkRedGlow.M_DarkRedGlow")
          (Rendering|Components|TextRender|SetTextRenderColor (Variables|Default|GetMove) (Variables|Default|GetSelected))
          (if (Utilities|String|Contains (Utilities|GetDisplayName self) "RPanel")
            (Default|ToRight (Variables|Default|GetCrane))
            (else
              (Default|ToLeft (Variables|Default|GetCrane)))))))))

(event EventBeginPlay
  (Variables|Default|SetButtonArr (Utilities|Array|MakeArray (Variables|Default|GetReleaseCube) (Variables|Default|GetGrabCube) (Variables|Default|GetMoveCube) 0))
  (Variables|Default|SetTextArr (Utilities|Array|MakeArray (Variables|Default|GetRelease) (Variables|Default|GetGrab) (Variables|Default|GetMove) (Variables|Default|GetTextRender)))
  (Variables|Default|SetUnselected (Class|KismetMathLibrary|LinearColortoRGBE (Class|KismetMathLibrary|LinearColorWhite)))
  (Variables|Default|SetSelected (Class|KismetMathLibrary|LinearColortoRGBE (Class|KismetMathLibrary|LinearColorBlack))))

(fn ConstructionScript)