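; BP_ServableWall is a breakable wall that shatters with a glass-breaking sound when its Served event is called, then dissolves and destroys itself.
; On BeginPlay it hides and deactivates its shard meshes, identified as static meshes whose names lack "Target" and "StaticMeshComponent0".
; Served swaps the intact mesh for physics-simulated shards with dynamic dissolve materials.
; After a short delay, a timeline drives their disFactor parameter before destroying the actor.
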(event EventBeginPlay
  (for _array_element (Actor|GetComponentsByClass "/Script/Engine.StaticMeshComponent")
    (if (!= (or (Utilities|String|Contains (Utilities|GetDisplayName _array_element) "Target") (Utilities|String|Contains (Utilities|GetDisplayName _array_element) "StaticMeshComponent0")) true)
      (Components|Activation|SetActive _array_element false false)
      (Physics|SetSimulatePhysics _array_element false)
      (Rendering|SetVisibility _array_element false false))))

(event EventServed
  (bind _staticmeshcomponent (Variables|Debug|GetStaticMeshComponent))
  (Audio|PlaySoundatLocation "/Game/Meshes/Glass_Breaking_Sound_Effect_HD___Glass_Shattering_Sound_Effect.Glass_Breaking_Sound_Effect_HD___Glass_Shattering_Sound_Effect" "0, 0, 0" "0, 0, 0" 1.0 1.0 0.0 0 0 0 0)
  (Rendering|SetVisibility _staticmeshcomponent false false)
  (Components|Activation|SetActive _staticmeshcomponent false false)
  (Collision|SetCollisionEnabled _staticmeshcomponent "NoCollision")
  (for _array_element (Actor|GetComponentsByClass "/Script/Engine.StaticMeshComponent")
    (if (!= (or (Utilities|String|Contains (Utilities|GetDisplayName _array_element) "Target") (Utilities|String|Contains (Utilities|GetDisplayName _array_element) "StaticMeshComponent0")) true)
      (Components|Activation|SetActive _array_element true false)
      (Physics|SetSimulatePhysics _array_element true)
      (Rendering|SetVisibility _array_element true false)
      (Rendering|Material|SetMaterial _array_element 0 "/Game/Materials/MI_BlackGlossDissolve.MI_BlackGlossDissolve")
      (bind _returnvalue (Rendering|Material|CreateDynamicMaterialInstance _array_element 0 (Rendering|Material|GetMaterial _array_element 0) "None" :!class /Script/Engine.PrimitiveComponent))
      (Utilities|Array|Add (Variables|Default|GetShards) _returnvalue)))
  (Utilities|FlowControl|Delay 2.0)
  (bind _disamount (Timeline|Timeline Play)
    (:Update
      (for _array_element_2 (Variables|Default|GetShards)
        (Rendering|Material|SetScalarParameterValue _array_element_2 "disFactor" _disamount :!class /Script/Engine.MaterialInstanceDynamic)))
    (:Finished
      (Actor|DestroyActor))))

(fn ConstructionScript)