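; Servant NPC that follows the player on foot and, when serving, AI-moves in flying mode to a target component.
; A spawned ServantDecoy_BP shadows its XY while stepping vertically toward target height, using a step derived from path length and speed.
; Arrival or overlap messages the target's owner via BPI_Servable, then the decoy descends and the servant rejoins the player's servants.
; Kill swaps it for a BreakableManInnit death actor.
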(event OnComponentBeginOverlap(CapsuleComponent)
  (params (OverlappedComponent :type Primitive%20Component%20Object%20Reference) (OtherActor :type Actor%20Object%20Reference) (OtherComp :type Primitive%20Component%20Object%20Reference) (OtherBodyIndex :type Integer) (bFromSweep :type Boolean) (SweepResult :type Hit%20Result%20Structure%20%28by%20ref%29))
  (bind _target (Variables|Default|GetTarget))
  (Utilities|IsValid _target
    (:Is%20Valid
      (if (or (== OtherComp _target) (== OtherActor (Components|GetOwner _target)))
        (CallFunction|ServeEnd)
        (Variables|Default|SetisServing false)))))

(event Custom|ServeStart
  (params (Index :type Integer))
  (bind _staticmesh (Variables|Default|GetStaticMesh))
  (bind _target (Variables|Default|GetTarget))
  (bind _staticmesh_2 (Variables|Default|GetStaticMesh))
  (bind _returnvalue (Transformation|GetWorldLocation _staticmesh))
  (bind _returnvalue_2 (Transformation|GetWorldLocation _target))
  (bind _returnvalue_3 (Transformation|GetWorldTransform _staticmesh_2))
  (Variables|Default|SetIndex (+ Index 1))
  (bind _returnvalue_4 (Class|NavigationSystemV1|FindPathtoLocationSynchronously _returnvalue (Math|Vector|MakeVector (.x _returnvalue_2) (.y _returnvalue_2) (.z _returnvalue_2)) (AI|GetAIController (Pawn|GetController)) 0))
  (Variables|Default|SetZStep (* (/ (.z (- (Math|Vector|MakeVector (.x _returnvalue_2) (.y _returnvalue_2) (.z _returnvalue_2)) _returnvalue)) (/ (Class|NavigationPath|GetPathLength _returnvalue_4) (Variables|/Script/Engine.CharacterMovementComponent|GetMaxFlySpeed (Variables|Character|GetCharacterMovement)))) 0.8))
  (bind _outactors (Actor|GetAllActorsOfClass "/Game/ServantDecoy_BP.ServantDecoy_BP_C"))
  (if (Utilities|Array|IsNotEmpty _outactors)
    (bind _array_element (Utilities|Array|ForEachLoopwithBreak _outactors :!label _label)
      (:LoopBody
        (if (Utilities|Array|ContainsItem (Variables|/Script/Engine.Actor|GetTags _array_element) (Utilities|String|StringToName (Utilities|String|BuildString(Integer) "DECOY" "" (Variables|Default|GetIndex))))
          (Actor|DestroyActor _array_element)
          (goto _label Break)))
      (:Completed
        (Utilities|IsValid (Variables|Default|GetDummy)
          (:Is%20Valid
            (Actor|DestroyActor (Variables|Default|GetDummy)))
          (:Is%20Not%20Valid
            _))
        (bind _returnvalue_5 (Game|SpawnActorfromClass "/Game/ServantDecoy_BP.ServantDecoy_BP_C" (Math|Transform|MakeTransform (.location _returnvalue_3) (.rotation _returnvalue_3) "1.000000,1.000000,1.000000") "Undefined" "MultiplyWithRoot" 0 0 :!label _label_2))
        (Default|SetData _returnvalue_5 self (Variables|Default|GetTarget))
        (Variables|Default|SetDummy _returnvalue_5)
        (Rendering|SetVisibility (Variables|Default|GetStaticMesh) true false)))
    (else
      (goto _label_2))))

(event Custom|ServeEnd
  (bind _target (Variables|Default|GetTarget))
  (bind _returnvalue (Components|GetOwner _target))
  (Utilities|IsValid _target
    (:Is%20Valid
      (if (Utilities|DoesObjectImplementInterface _returnvalue "/Game/BPI_Servable.BPI_Servable_C")
        (Class|BPIServable|Served(Message) _returnvalue)
        (Variables|Default|SetisServing false)))))

(event EventBeginPlay
  (bind _returnvalue (Actor|GetActorOfClass "/Game/FirstPersonBP1/Blueprints/BP_FirstPersonCharacter.BP_FirstPersonCharacter_C"))
  (Variables|Default|SetPlayerBP _returnvalue))

(event EventTick
  (params (DeltaSeconds :type Float%20%28single-precision%29))
  (bind _target (Variables|Default|GetTarget))
  (bind _staticmesh (Variables|Default|GetStaticMesh))
  (bind _dummy (Variables|Default|GetDummy))
  (bind _staticmesh_2 (Variables|Default|GetStaticMesh))
  (bind _dummy_2 (Variables|Default|GetDummy))
  (bind _staticmesh_3 (Variables|Default|GetStaticMesh))
  (bind _playerbp (Variables|Default|GetPlayerBP))
  (bind _returnvalue (Transformation|GetWorldLocation _target))
  (bind _returnvalue_2 (Transformation|GetWorldLocation _staticmesh_3))
  (bind _returnvalue_3 (Transformation|GetWorldLocation _staticmesh))
  (bind _returnvalue_4 (Transformation|GetWorldRotation _staticmesh_2))
  (bind _rootcomponent (Variables|/Script/Engine.Actor|GetRootComponent _dummy))
  (bind _staticmeshcomponent (Variables|/Script/Engine.StaticMeshActor|GetStaticMeshComponent _dummy_2))
  (bind _returnvalue_5 (Transformation|GetWorldLocation _staticmeshcomponent))
  (bind _returnvalue_6 (Transformation|GetWorldLocation _rootcomponent))
  (if (Variables|Default|GetisServing)
    (Pawn|Components|CharacterMovement|SetMovementMode (Variables|Character|GetCharacterMovement) "MOVE_Flying" 0)
    (AI|AIMoveTo (AI|GetAIController (Pawn|GetController)) (Transformation|GetWorldLocation (Variables|Default|GetTarget)) 0 -1.0 "Disable" "Enable" true true
      (:then
        (Utilities|IsValid _dummy
          (:Is%20Valid
            (Utilities|IsValid _target
              (:Is%20Valid
                (if (< (.z _returnvalue_6) (.z _returnvalue))
                  (Transformation|SetWorldLocation _rootcomponent (Math|Vector|MakeVector (.x _returnvalue_3) (.y _returnvalue_3) (+ (.z _returnvalue_6) (Variables|Default|GetZStep))) false false)
                  (else
                    (Transformation|SetWorldLocation _rootcomponent (Math|Vector|MakeVector (.x _returnvalue_3) (.y _returnvalue_3) (.z _returnvalue)) false false)))
                (Transformation|SetActorRotation _dummy (Math|Rotator|MakeRotator (.roll _returnvalue_4) (.pitch _returnvalue_4) (+ (.yaw _returnvalue_4) 9e+01))))
              (:Is%20Not%20Valid
                (Development|PrintString "INVALID TARGET"))))
          (:Is%20Not%20Valid
            (Variables|Default|SetisServing false)
            (Development|PrintString "INVALID DUMMY"))))
      (:OnRequestFailed
        (Development|PrintString "FAILED"))
      (:OnMoveFinished
        (CallFunction|ServeEnd)))
    (else
      (Utilities|IsValid (Variables|Default|GetDummy)
        (:Is%20Valid
          (if (> (.z _returnvalue_5) (.z _returnvalue_2))
            (Transformation|SetWorldLocation _staticmeshcomponent (Math|Vector|MakeVector (.x _returnvalue_2) (.y _returnvalue_2) (- (.z _returnvalue_5) 5.0)) false false)
            (else
              (Actor|DestroyActor (Variables|Default|GetDummy))
              (Rendering|SetVisibility (Variables|Default|GetStaticMesh) true false)
              (Default|AddServant (Variables|Default|GetPlayerBP) self))))
        (:Is%20Not%20Valid
          ;[0.15 0.15 0.15 0.5] Follow Player!
          (Pawn|Components|CharacterMovement|SetMovementMode (Variables|Character|GetCharacterMovement) "MOVE_Walking" 0)
          (Utilities|FlowControl|DoOnce false :!label _label
            (:Completed
              (Transformation|SetActorRotation (Math|Conversions|RotationFromXVector (- (Transformation|GetActorLocation _playerbp) (Transformation|GetActorLocation))))
              (AI|AIMoveTo (AI|GetAIController (Pawn|GetController)) "0, 0, 0" _playerbp 2.5e+02 "Default" "Default" true true
                (:OnMoveFinished
                  (goto _label Reset))))))))))

(fn ConstructionScript)

(fn Kill
  (bind _returnvalue (Game|SpawnActorfromClass "/Game/Meshes/BreakableManInnit.BreakableManInnit_C" (Transformation|GetActorTransform) "AlwaysSpawn" "MultiplyWithRoot" 0 0))
  (Default|Death _returnvalue)
  (Actor|DestroyActor))

(fn Activate)