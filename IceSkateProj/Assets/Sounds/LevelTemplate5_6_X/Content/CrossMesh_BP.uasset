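; CrossMesh_BP is an attachment spot where a horse part actor snaps into place.
; Activate reveals MorseHesh, and when an actor whose display name contains "HorseParts" overlaps it while visible, MorseHesh swaps to HorseMesh and that actor is destroyed.
; A second later it calls CallEDCross.
; A separate Fade event drives a supplied image's opacity through a timeline, then reverses it after a short pause.
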(event OnComponentBeginOverlap(MorseHesh)
  (params (OverlappedComponent :type Primitive%20Component%20Object%20Reference) (OtherActor :type Actor%20Object%20Reference) (OtherComp :type Primitive%20Component%20Object%20Reference) (OtherBodyIndex :type Integer) (bFromSweep :type Boolean) (SweepResult :type Hit%20Result%20Structure%20%28by%20ref%29))
  (if (and (Utilities|String|Contains (Utilities|GetDisplayName OtherActor) "HorseParts") (Rendering|IsVisible (Variables|Default|GetMorseHesh)))
    (CallFunction|Attatched)
    (Actor|DestroyActor OtherActor)
    (Utilities|FlowControl|Delay 1.0)
    (Default|CallEDCross)))

(event Custom|Activate
  (Rendering|SetVisibility (Variables|Default|GetMorseHesh) true false))

(event Custom|Attatched
  (Rendering|SetVisibility (Variables|Default|GetMorseHesh) false false)
  (Rendering|SetVisibility (Variables|Default|GetHorseMesh) true false))

(event Custom|Fade
  (params (HUD :type Anim%20HUD%20BP%20Object%20Reference) (Image :type Image%20Object%20Reference))
  (bind _opacity (Timeline|Timeline Play)
    (:Update
      (Class|Image|SetOpacity Image _opacity))
    (:Finished
      (Utilities|FlowControl|Delay 1.0)
      (Timeline|Timeline Reverse))))

(fn ConstructionScript)