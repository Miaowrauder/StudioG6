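; BP_MulchoMatic is a puzzle machine that takes in a basket pickup, produces Holy Mulch and releases the shutter doors.
; The Mulcher overlap identifies baskets by a display-name substring, then hides and disables the overlapping component.
; On the first match only, it switches its indicator lights and spawns HolyMulch_Blueprint at its StaticMesh.
; It then calls Fall and LightSwitch on every BP_ShutterDoor and disables their collision.
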(event OnComponentBeginOverlap(Mulcher)
  (params (OverlappedComponent :type Primitive%20Component%20Object%20Reference) (OtherActor :type Actor%20Object%20Reference) (OtherComp :type Primitive%20Component%20Object%20Reference) (OtherBodyIndex :type Integer) (bFromSweep :type Boolean) (SweepResult :type Hit%20Result%20Structure%20%28by%20ref%29))
  (if (Utilities|String|Contains (Utilities|GetDisplayName OtherComp) "BP_BasketPickup")
    (Rendering|SetVisibility OtherComp false false)
    (Physics|SetSimulatePhysics OtherComp false)
    (Collision|SetCollisionEnabled OtherComp "NoCollision")
    (Components|Activation|SetActive OtherComp false false)
    (Utilities|FlowControl|DoOnce false
      (:Completed
        (CallFunction|LightSwitch)
        (Game|SpawnActorfromClass "/Game/HolyMulch_Blueprint.HolyMulch_Blueprint_C" (Math|Transform|MakeTransform (Transformation|GetWorldLocation (Variables|Default|GetStaticMesh)) "0, 0, 0" "1.000000,1.000000,1.000000") "AlwaysSpawn" "MultiplyWithRoot" 0 0)
        (bind _outactors (Actor|GetAllActorsOfClass "/Game/Blueprints/BP_ShutterDoor.BP_ShutterDoor_C"))
        (for _array_element _outactors
          (Default|Fall _array_element)
          (Default|LightSwitch _array_element)
          (Collision|SetCollisionEnabled (Variables|/Game/Blueprints/BP_ShutterDoor.BP_ShutterDoor_C|GetDoor _array_element) "NoCollision"))))))

(event Custom|LightSwitch
  (Rendering|Material|SetMaterial (Variables|Default|GetGreenLight) 1 "/Game/Materials/M_GlowDarkGreyNavy.M_GlowDarkGreyNavy")
  (Rendering|Components|Light|SetIntensity (Variables|Default|GetPointLight) 5e+02)
  (Rendering|Material|SetMaterial (Variables|Default|GetRedLight) 1 "/Game/Materials/M_FlatBlack.M_FlatBlack")
  (Rendering|Components|Light|SetIntensity (Variables|Default|GetPointLight1) 5e+02))

(fn ConstructionScript)