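; Parent Blueprint for fracture slab actors, handling their text labels and enabling input from player 0 on BeginPlay.
; A 0.2-second Delay loop turns TextRender to face the player camera, changing yaw only so the text stays upright.
; When TextStillActive is false, the loop ends and destroys the TextRender and TextRender1 components.
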(event EventBeginPlay
  ;[1 1 1] Text
  (Input|EnableInput (Game|GetPlayerController 0))
  (Utilities|FlowControl|Delay 0.2 :!label _label)
  (Transformation|SetRelativeRotation (Variables|Default|GetTextRender) (Math|Rotator|MakeRotator 0.0 0.0 (.yaw (Math|Conversions|RotationFromXVector (- (Transformation|GetActorLocation (Game|GetPlayerCameraManager 0)) (Transformation|GetWorldLocation (Variables|Default|GetTextRender)))))) false false)
  (if (Variables|Default|GetTextStillActive?)
    (goto _label)
    (else
      (Components|DestroyComponent (Variables|Default|GetTextRender)))))

(fn ConstructionScript)