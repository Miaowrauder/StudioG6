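; BP_LazerDoor is a laser barrier door that exposes events to open and break it, with no trigger logic of its own.
; LightSwitch turns the red light off and the green light on.
; Fall hides and deactivates the four lasers and removes collision from them and the door parts.
; Destroy plays a fracture sound at the world origin and destroys the Light and Left components.
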(event Custom|Fall
  (bind _laser3 (Variables|Default|GetLaser3))
  (Rendering|SetVisibility (Variables|Default|GetLaser) false false)
  (Components|Activation|SetActive _laser3 false false)
  (Collision|SetCollisionEnabled _laser3 "NoCollision"))

(event Custom|LightSwitch
  (Rendering|Components|Light|SetIntensity (Variables|Default|GetGreen) 1e+05)
  (Rendering|Components|Light|SetIntensity (Variables|Default|GetRed) 0.0))

(event Custom|Destroy
  (Audio|PlaySoundatLocation "/Game/SFX/Fracture2.Fracture2" "0, 0, 0" "0, 0, 0" 1.0 1.0 0.0 0 0 0 0)
  (Components|DestroyComponent (Variables|Default|GetLight)))

(fn ConstructionScript)